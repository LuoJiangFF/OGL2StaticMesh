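; Test Blueprint that builds a static mesh at runtime from a saved .ogl file and checks mouse picking on spawned actors.
; On BeginPlay it loads a hard-coded file's bytes into a C++ NewStaticMesh call and shows the result on a spawned, scaled-up actor.
; It also spawns a default Cube with a dynamic AliasMaster material.
; Left click line-traces from the cursor and prints the hit actor.
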(event `self.ReceiveBeginPlay`
  (bind _spawn_transform (`self.Spawn Transform`))
  (set `PlayerController.bShowMouseCursor` true (`GameplayStatics.GetPlayerController` 0))
  (`|ExecutionSequence`
    (:`then_0`
      ;[1 1 1] OGL2Mesh
      (bind _returnvalue (`|SpawnActorFromClass` "/Script/Engine.Actor" _spawn_transform "Undefined" "OverrideRootScale" null null))
      (bind _returnvalue_2 (`AddComponent|NODE_AddStaticMeshComponent-2` :`self` _returnvalue :`RelativeTransform` _spawn_transform))
      (`self.K2_AddActorLocalTransform` _returnvalue (`KismetMathLibrary.MakeTransform` (38216.597656 37783.464844 5016.76709) (struct) (100.0 100.0 100.0)) false false)
      (bind _result (`BaseFilesDownloader.LoadFileToArray` (`KismetStringLibrary.Concat_StrStr` (`KismetSystemLibrary.GetProjectSavedDirectory`) "OGL/" "118442645" ".ogl")))
      ;;[1 1 1] Load OGL File To StaticMesh
      (bind _returnvalue_3 (`PixelsBlueprintFunctionLibrary.NewStaticMesh` "" (`self.S Mat`) 100000 (`|GetArrayItem` _result) (`KismetArrayLibrary.Array_Length` _result))) ; C++ Script
      (bind _returnvalue_4 (`StaticMeshComponent.SetStaticMesh` _returnvalue_2 _returnvalue_3)))
    (:`then_1`
      ;[1 1 1] Default
      (bind _returnvalue_5 (`|SpawnActorFromClass` "/Script/Engine.Actor" _spawn_transform "Undefined" "OverrideRootScale" null null))
      (bind _returnvalue_6 (`AddComponent|NODE_AddStaticMeshComponent-1` :`self` _returnvalue_5 :`RelativeTransform` _spawn_transform))
      (`self.K2_AddActorLocalTransform` _returnvalue_5 (`KismetMathLibrary.MakeTransform` (38354.597656 37547.464844 5016.76709)) false false)
      (bind _returnvalue_7 (`StaticMeshComponent.SetStaticMesh` _returnvalue_6 "/Engine/BasicShapes/Cube.Cube"))
      (if _returnvalue_7
        (bind _returnvalue_8 (`KismetMaterialLibrary.CreateDynamicMaterialInstance` "/DatasmithContent/Materials/AliasMaster.AliasMaster"))
        (`PrimitiveComponent.SetMaterial` _returnvalue_6 0 _returnvalue_8)))))

(event `Key|LeftMouseButton`
  (params (Key :type "Key Structure"))
  (bind (_worldlocation _worlddirection) (`PlayerController.DeprojectMousePositionToWorld` (`GameplayStatics.GetPlayerController` 0)))
  (bind _returnvalue (+ _worldlocation (* _worlddirection 200000.0)))
  ;[1 1 1] Click Actor Test
  (:`Pressed`
    (`KismetSystemLibrary.PrintString` (`KismetStringLibrary.Conv_VectorToString` _worldlocation))
    (`KismetSystemLibrary.PrintString` (`KismetStringLibrary.Conv_VectorToString` _returnvalue))
    (bind (_outhit _returnvalue_2) (`KismetSystemLibrary.LineTraceSingle` :`Start` _worldlocation :`End` _returnvalue :`TraceChannel` "TraceTypeQuery1" :`bTraceComplex` true :`DrawTime` 0.0))
    (if _returnvalue_2
      (`KismetSystemLibrary.PrintString` (`KismetSystemLibrary.GetDisplayName` (`.HitActor` (`GameplayStatics.BreakHitResult` _outhit))))
      (else
        (`KismetSystemLibrary.PrintString` (`KismetStringLibrary.Conv_BoolToString` _returnvalue_2))))))

(fn `UserConstructionScript`)